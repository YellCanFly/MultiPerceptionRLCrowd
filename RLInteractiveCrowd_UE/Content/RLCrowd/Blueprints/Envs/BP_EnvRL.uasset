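; Environment actor for a reinforcement-learning crowd simulation, with a main UI widget, a key-nudged camera and a 30 FPS cap.
; Construction sizes four boundary cubes and the floor plane from EnvConfig, then initializes an implicit-environment texture from a name-keyed library.
; Environment resets push that texture into the plane's dynamic material.
; Helper functions record per-agent status snapshots and export them to timestamped JSON files named by environment and reward weights.
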(event `self.ReceiveBeginPlay`
  (bind _returnvalue (`GameplayStatics.GetPlayerController` 0))
  (`|ExecutionSequence`
    (:`then_0`
      (`self.EnableInput` _returnvalue)
      (set `PlayerController.bShowMouseCursor` true _returnvalue)
      (set `PlayerController.bEnableClickEvents` true _returnvalue)
      (set `PlayerController.bEnableMouseOverEvents` true _returnvalue)
      (`PlayerController.SetViewTargetWithBlend` _returnvalue self 0.0 "VTBlend_Linear" 0.0 false)
      (bind _returnvalue_2 (`|CreateWidget` "/Game/RLCrowd/Blueprints/UI/WBP_Main_RL.WBP_Main_RL_C" _returnvalue))
      (bind _output_get (set `self.WBP_Main` _returnvalue_2))
      (`UserWidget.AddToViewport` _output_get 0)
      (`KismetSystemLibrary.ExecuteConsoleCommand` "t.MaxFPS 30" (`GameplayStatics.GetPlayerController` 0)))
    (:`then_1`
      (add `self.OnEnvReset` (delegate `UpdateResetVisulize`)))))

(event `UpdateResetVisulize`
  (`/Engine/EditorBlueprintResources/StandardMacros.IsValid` (`self.implicit_env_texture`)
    (:`Is Valid`
      (`MaterialInstanceDynamic.SetTextureParameterValue` (`self.TerrainDynamicMat`) "Texture" (`self.implicit_env_texture`)))))

(event `Key|Left`
  (params (Key :type "Key Structure"))
  ;[1 1 1] Control Camera
  (:`Pressed`
    (`SceneComponent.K2_AddLocalOffset` (`self.Camera`) (0.0 -20.0 0.0) false false)))

(event `Key|Up`
  (params (Key :type "Key Structure"))
  ;[1 1 1] Control Camera
  (:`Pressed`
    (`SceneComponent.K2_AddLocalOffset` (`self.Camera`) (0.0 0.0 20.0) false false)))

(event `Key|Equals`
  (params (Key :type "Key Structure"))
  ;[1 1 1] Control Camera
  (:`Pressed`
    (`SceneComponent.K2_AddLocalOffset` (`self.Camera`) (20.0 0.0 0.0) false false)))

(event `Key|Right`
  (params (Key :type "Key Structure"))
  ;[1 1 1] Control Camera
  (:`Pressed`
    (`SceneComponent.K2_AddLocalOffset` (`self.Camera`) (0.0 20.0 0.0) false false)))

(event `Key|Down`
  (params (Key :type "Key Structure"))
  ;[1 1 1] Control Camera
  (:`Pressed`
    (`SceneComponent.K2_AddLocalOffset` (`self.Camera`) (0.0 0.0 -20.0) false false)))

(event `Key|Hyphen`
  (params (Key :type "Key Structure"))
  ;[1 1 1] Control Camera
  (:`Pressed`
    (`SceneComponent.K2_AddLocalOffset` (`self.Camera`) (-20.0 0.0 0.0) false false)))

(event `self.update_env_vis`
  (bind (_env_size_x _env_size_y) (`KismetMathLibrary.BreakVector2D` (`self.env_size`)))
  (bind (_env_size_x_2 _env_size_y_2) (`KismetMathLibrary.BreakVector2D` (`self.env_size`)))
  (bind _env_size_x_3 (`KismetMathLibrary.BreakVector2D` (`self.env_size`)))
  (bind (_env_size_x_4 _env_size_y_3) (`KismetMathLibrary.BreakVector2D` (`self.env_size`)))
  (bind (_env_size_x_5 _env_size_y_4) (`KismetMathLibrary.BreakVector2D` (`self.env_size`)))
  (bind _env_size_x_6 (`KismetMathLibrary.BreakVector2D` (`self.env_size`)))
  (bind (_env_size_x_7 _env_size_y_5) (`KismetMathLibrary.BreakVector2D` (`self.env_size`)))
  (bind _env_size_x_8 (`KismetMathLibrary.BreakVector2D` (`self.env_size`)))
  (bind _returnvalue (* _env_size_x_3 50.0))
  (bind _returnvalue_2 (* _env_size_y_4 50.0))
  ;[1 1 1] UpdateVisulize
  (`|ExecutionSequence`
    (:`then_0`
      (`SceneComponent.SetRelativeScale3D` (`self.Cube1`) (`KismetMathLibrary.MakeVector` _env_size_x_8 0.05 1.0))
      (`SceneComponent.SetRelativeScale3D` (`self.Cube3`) (`KismetMathLibrary.MakeVector` _env_size_x_8 0.05 1.0))
      (`SceneComponent.K2_SetRelativeLocation` (`self.Cube1`) (`KismetMathLibrary.MakeVector` _returnvalue) false false)
      (`SceneComponent.K2_SetRelativeLocation` (`self.Cube3`) (`KismetMathLibrary.MakeVector` _returnvalue (* _env_size_y_2 100.0)) false false))
    (:`then_1`
      (`SceneComponent.SetRelativeScale3D` (`self.Cube2`) (`KismetMathLibrary.MakeVector` 0.05 _env_size_y_5 1.0))
      (`SceneComponent.SetRelativeScale3D` (`self.Cube4`) (`KismetMathLibrary.MakeVector` 0.05 _env_size_y_5 1.0))
      (`SceneComponent.K2_SetRelativeLocation` (`self.Cube2`) (`KismetMathLibrary.MakeVector` 0.0 _returnvalue_2) false false)
      (`SceneComponent.K2_SetRelativeLocation` (`self.Cube4`) (`KismetMathLibrary.MakeVector` (* _env_size_x_6 100.0) _returnvalue_2) false false))
    (:`then_2`
      (`SceneComponent.K2_SetRelativeLocation` (`self.EnvCenter`) (`KismetMathLibrary.MakeVector` (* _env_size_x 50.0) (* _env_size_y 50.0)) false false)
      (`SceneComponent.SetRelativeScale3D` (`self.Plane`) (`KismetMathLibrary.MakeVector` _env_size_x_4 _env_size_y_3 1.0)))))

(fn `save_agents_status_to_file`
  (returns (Success :type Boolean))
  (bind (_returnvalue_hours _returnvalue_minutes _returnvalue_seconds) (break `Timecode` (`TimeManagementBlueprintLibrary.GetTimecode`)))
  (bind _recordagentstatuses (`self.RecordAgentStatuses`))
  (bind (_alive_penalty _velocity_smooth_penalty _collision_penalty _target_approach_distance_reward _target_away_distance_penalty_ratio _nav_point_approach_distance_reward _target_arrive_reward _obstacle_penalty _obstacle_time_coef _implicit_env_penalty _reward_weight_entity_low _reward_weight_entity_up _reward_weight_implicit_low _reward_weight_implicit_up) (break `S_RewardConfig` (`self.reward_config`)))
  (bind _returnvalue (`KismetStringLibrary.Concat_StrStr` (`KismetSystemLibrary.GetProjectDirectory`) "/../../record_agent_status/" (`KismetStringLibrary.Concat_StrStr` (`.env_title` (break `S_EnvConfig` (`self.env_config`))) (`KismetTextLibrary.Conv_TextToString` (`|FormatText` "_env_{env_name}_entity_{we}_implicit_{wi}" (`.implicit_env_texture_name` (break `S_EnvConfig` (`self.env_config`))) _reward_weight_entity_low _reward_weight_implicit_up)) "_" (`KismetTextLibrary.Conv_TextToString` (`|FormatText` "{h}_{m}_{s}" _returnvalue_hours _returnvalue_minutes _returnvalue_seconds))) ".json"))
  (`KismetSystemLibrary.PrintString` (`KismetStringLibrary.Conv_IntToString` (`KismetArrayLibrary.Array_Length` _recordagentstatuses)) true true (struct :`R` 1.0 :`B` 0.082829 :`A` 1.0) 20.0)
  (bind _outjsonstring (`|StructToJsonString` (make `/Game/RLCrowd/Blueprints/Struct/S_AgentStatusInOneEval` _recordagentstatuses)))
  (bind _outjsonobject (`JsonBlueprintFunctionLibrary.FromString` _outjsonstring))
  (`KismetSystemLibrary.PrintString` _returnvalue true true (struct :`R` 0.140625 :`G` 0.239022 :`B` 1.0 :`A` 1.0) 20.0)
  (bind _returnvalue_2 (`JsonBlueprintFunctionLibrary.ToFile` _outjsonobject (make `FilePath` _returnvalue)))
  (return _returnvalue_2))

(fn `save_current_agents_status`
  (locals (AgentStatusTemp :type "Array of /Game/RLCrowd/Blueprints/Struct/S_AgentStatus Structure"))
  (`KismetArrayLibrary.Array_Clear` (`local.AgentStatusTemp`))
  (for _array_element (`self.agents`)
    (`KismetArrayLibrary.Array_Add` (`local.AgentStatusTemp`) (make `/Game/RLCrowd/Blueprints/Struct/S_AgentStatus` (`AgentBase.index` _array_element) (`AgentBase.position` _array_element) (`AgentBase.velocity` _array_element) (`AgentBase.orientation` _array_element) (`AgentRL.implicit_env_value` _array_element))))
  (`KismetArrayLibrary.Array_Add` (`self.RecordAgentStatuses`) (make `/Game/RLCrowd/Blueprints/Struct/S_AgentStatus2D` (`local.AgentStatusTemp`))))

(fn `UserConstructionScript`
  (bind _plane (`self.Plane`))
  (bind (_env_type _env_title _width _height) (break `S_EnvConfig` (`self.env_config`)))
  (bind _returnvalue (`PrimitiveComponent.CreateDynamicMaterialInstance` _plane 0 (`PrimitiveComponent.GetMaterial` _plane 0) "None"))
  (set `self.TerrainDynamicMat` _returnvalue)
  (`self.update_env_vis`)
  (for _array_element (`self.TerrainTextureLib`)
    (`BlueprintMapLibrary.Map_Add` (`self.implicit_env_texture_dict`) (`KismetSystemLibrary.GetObjectName` _array_element) _array_element))
  (set `self.implicit_env_texture` (`BlueprintMapLibrary.Map_Find` (`self.implicit_env_texture_dict`) "white"))
  (set `self.env_size` (`KismetMathLibrary.MakeVector2D` _width _height))
  (`self.update_env_vis`)
  (`self.init_implicit_env_texture`))