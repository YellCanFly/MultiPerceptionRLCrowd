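; Hallway environment for RL crowd agents, spawning two opposing groups that must cross the space.
; AddNewAgents splits NumAgents into two evenly spaced rows at mirrored Y positions, each agent targeting the same X on the opposite row.
; Each agent is initialized from EnvConfig and RewardConfig, starts at zero velocity, references this environment and joins the Agents list.
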(event `self.add_new_agents`
  (bind (_env_size_x _env_size_y) (`KismetMathLibrary.BreakVector2D` (`self.env_size`)))
  (bind (_env_size_x_2 _env_size_y_2) (`KismetMathLibrary.BreakVector2D` (`self.env_size`)))
  (bind _env_size_x_3 (`KismetMathLibrary.BreakVector2D` (`self.env_size`)))
  (bind (_env_size_x_4 _env_size_y_3) (`KismetMathLibrary.BreakVector2D` (`self.env_size`)))
  (bind (_env_size_x_5 _env_size_y_4) (`KismetMathLibrary.BreakVector2D` (`self.env_size`)))
  (bind _env_size_x_6 (`KismetMathLibrary.BreakVector2D` (`self.env_size`)))
  (bind _env_size_x_7 (`KismetMathLibrary.BreakVector2D` (`self.env_size`)))
  (bind _env_size_x_8 (`KismetMathLibrary.BreakVector2D` (`self.env_size`)))
  (bind (_env_type _env_title _width _height _implicit_env_texture_name _num_agents _target_loc_margin _agent_radius _num_rays _max_ray_distance _ray_vision_lamda _max_speed_orientation _max_speed_perpendicular _max_acceleration _max_angular_velocity _dt _action_interval_step_num _min_walking_distance _max_alive_time _arrive_range_scale _max_time_overlaped_with_obstacle _implicit_env_obs_range _implicit_env_value_threshold _implicit_agent_spawn_threshold _implicit_agent_target_threshold _use_nav_point _update_nav_point_threshold) (break `S_EnvConfig` (`self.env_config`)))
  (bind (_env_type_2 _env_title_2 _width_2 _height_2 _implicit_env_texture_name_2 _num_agents_2 _target_loc_margin_2 _agent_radius_2 _num_rays_2 _max_ray_distance_2 _ray_vision_lamda_2 _max_speed_orientation_2 _max_speed_perpendicular_2 _max_acceleration_2 _max_angular_velocity_2 _dt_2 _action_interval_step_num_2 _min_walking_distance_2 _max_alive_time_2 _arrive_range_scale_2 _max_time_overlaped_with_obstacle_2 _implicit_env_obs_range_2 _implicit_env_value_threshold_2 _implicit_agent_spawn_threshold_2 _implicit_agent_target_threshold_2 _use_nav_point_2 _update_nav_point_threshold_2) (break `S_EnvConfig` (`self.env_config`)))
  (`|ExecutionSequence`
    (:`then_0`
      ;[1 1 1] 重新生成Agents
      (for _index (range (/ (`self.num_agents`) 2))
        (bind _returnvalue (`|SpawnActorFromClass` (`self.AgentRLClass`) (`KismetMathLibrary.MakeTransform` (0.0 0.0 0.0)) "Undefined" "OverrideRootScale" null null))
        (bind _returnvalue_2 (+ (* _env_size_x_7 (* (- 1.0 (`self.XSpawnRangeRatio`)) 0.5)) (* _index (/ (* _env_size_x_6 (`self.XSpawnRangeRatio`)) (- (/ (`self.num_agents`) 2) 1)))))
        (`AgentRL.init_agent_rl` _returnvalue (make `S_AgentConfig` _index (`KismetMathLibrary.MakeVector2D` _returnvalue_2 (* _env_size_y_3 (`self.YSpawnLocRatio`))) (`KismetMathLibrary.MakeVector2D` _returnvalue_2 (* _env_size_y_4 (- 1.0 (`self.YSpawnLocRatio`)))) _agent_radius_2 _num_rays_2 _max_ray_distance_2 _ray_vision_lamda_2 _max_speed_orientation_2 _max_speed_perpendicular_2 _max_acceleration_2 _max_angular_velocity_2 _dt_2 _max_alive_time_2 _arrive_range_scale_2 _max_time_overlaped_with_obstacle_2 _implicit_env_obs_range_2 _implicit_env_value_threshold_2 _use_nav_point_2 _update_nav_point_threshold_2 (`self.reward_config`)))
        (set `AgentBase.velocity` (0.0 0.0) _returnvalue)
        (set `AgentRL.env` self _returnvalue)
        (`KismetArrayLibrary.Array_Add` (`self.agents`) _returnvalue)))
    (:`then_1`
      ;[1 1 1] 重新生成Agents
      (for _index_2 (range (/ (`self.num_agents`) 2))
        (bind _returnvalue_3 (`|SpawnActorFromClass` (`self.AgentRLClass`) (`KismetMathLibrary.MakeTransform` (0.0 0.0 0.0)) "Undefined" "OverrideRootScale" null null))
        (bind _returnvalue_4 (+ (* _env_size_x_3 (* (- 1.0 (`self.XSpawnRangeRatio`)) 0.5)) (* _index_2 (/ (* _env_size_x_8 (`self.XSpawnRangeRatio`)) (- (/ (`self.num_agents`) 2) 1)))))
        (`AgentRL.init_agent_rl` _returnvalue_3 (make `S_AgentConfig` (+ _index_2 (/ (`self.num_agents`) 2)) (`KismetMathLibrary.MakeVector2D` _returnvalue_4 (* _env_size_y_2 (- 1.0 (`self.YSpawnLocRatio`)))) (`KismetMathLibrary.MakeVector2D` _returnvalue_4 (* _env_size_y (`self.YSpawnLocRatio`))) _agent_radius _num_rays _max_ray_distance _ray_vision_lamda _max_speed_orientation _max_speed_perpendicular _max_acceleration _max_angular_velocity _dt _max_alive_time _arrive_range_scale _max_time_overlaped_with_obstacle _implicit_env_obs_range _implicit_env_value_threshold _use_nav_point _update_nav_point_threshold (`self.reward_config`)))
        (set `AgentBase.velocity` (0.0 0.0) _returnvalue_3)
        (set `AgentRL.env` self _returnvalue_3)
        (`KismetArrayLibrary.Array_Add` (`self.agents`) _returnvalue_3))
      (set `self.newest_agent_index` (`self.num_agents`)))))

(fn `UserConstructionScript`
  (`parent.UserConstructionScript`))