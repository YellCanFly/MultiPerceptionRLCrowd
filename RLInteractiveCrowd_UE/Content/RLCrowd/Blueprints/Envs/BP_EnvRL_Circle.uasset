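; Reinforcement-learning crowd environment that sets up a circle-crossing scenario for RL agents.
; AddNewAgents spawns NumAgents evenly around a circle at the environment's centre, each targeting the diametrically opposite point.
; Each agent is initialised from the shared EnvConfig and RewardConfig, given zero velocity and a reference to this environment, then added to Agents.
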(event `self.add_new_agents`
  (bind _envcircleradius (`self.EnvCircleRadius`))
  (bind (_env_type _env_title _width _height _implicit_env_texture_name _num_agents _target_loc_margin _agent_radius _num_rays _max_ray_distance _ray_vision_lamda _max_speed_orientation _max_speed_perpendicular _max_acceleration _max_angular_velocity _dt _action_interval_step_num _min_walking_distance _max_alive_time _arrive_range_scale _max_time_overlaped_with_obstacle _implicit_env_obs_range _implicit_env_value_threshold _implicit_agent_spawn_threshold _implicit_agent_target_threshold _use_nav_point _update_nav_point_threshold) (break `S_EnvConfig` (`self.env_config`)))
  (bind _returnvalue (* (`self.env_size`) (0.5 0.5)))
  ;[1 1 1] 重新生成Agents
  (for _index (range (`self.num_agents`))
    (bind _returnvalue_2 (`|SpawnActorFromClass` (`self.AgentRLClass`) (`KismetMathLibrary.MakeTransform` (0.0 0.0 0.0)) "Undefined" "OverrideRootScale" null null))
    (bind _returnvalue_3 (* _index (/ 360.0 (`KismetMathLibrary.Conv_IntToDouble` (`self.num_agents`)))))
    (bind _returnvalue_4 (mod (+ _returnvalue_3 180.0) 360.0))
    (`AgentRL.init_agent_rl` _returnvalue_2 (make `S_AgentConfig` _index (+ (* (`KismetMathLibrary.MakeVector2D` (`KismetMathLibrary.DegCos` _returnvalue_3) (`KismetMathLibrary.DegSin` _returnvalue_3)) (`KismetMathLibrary.MakeVector2D` _envcircleradius _envcircleradius)) _returnvalue) (+ _returnvalue (* (`KismetMathLibrary.MakeVector2D` (`KismetMathLibrary.DegCos` _returnvalue_4) (`KismetMathLibrary.DegSin` _returnvalue_4)) (`KismetMathLibrary.MakeVector2D` _envcircleradius _envcircleradius))) _agent_radius _num_rays _max_ray_distance _ray_vision_lamda _max_speed_orientation _max_speed_perpendicular _max_acceleration _max_angular_velocity _dt _max_alive_time _arrive_range_scale _max_time_overlaped_with_obstacle _implicit_env_obs_range _implicit_env_value_threshold _use_nav_point _update_nav_point_threshold (`self.reward_config`)))
    (set `AgentBase.velocity` (0.0 0.0) _returnvalue_2)
    (set `AgentRL.env` self _returnvalue_2)
    (`KismetArrayLibrary.Array_Add` (`self.agents`) _returnvalue_2))
  (set `self.newest_agent_index` (`self.num_agents`)))

(fn `UserConstructionScript`
  (`parent.UserConstructionScript`))