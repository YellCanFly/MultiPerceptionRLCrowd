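; Crowd replay actor that visualizes recorded RL agent episodes as third-person characters.
; Space plays a range of JSON records in sequence, advancing one frame per gated Tick; Left/Right step frames manually.
; Each frame spawns, moves or destroys characters through agent-ID maps, setting velocity and converting positions to centimeters at fixed height.
; The construction script applies the chosen environment's mask texture and shows either a ground plane or the landscape.
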(event `ReadData`
  (params (DataFileName :type String))
  ;[1 1 1] Read data
  (bind _outjsonobject (`JsonBlueprintFunctionLibrary.FromFile` (make `FilePath` (`KismetStringLibrary.Concat_StrStr` (`KismetSystemLibrary.GetProjectDirectory`) "/../../record_agent_status/" DataFileName ".json"))))
  (bind _outvalue (`|GetJsonField` _outjsonobject "frames"))
  (set `self.Frames` _outvalue)
  (`KismetArrayLibrary.Array_Clear` (`self.AgentMaps`))
  (`KismetArrayLibrary.Array_Resize` (`self.AgentMaps`) (`KismetArrayLibrary.Array_Length` (`self.Frames`)))
  (for (_array_element _array_index) (`self.Frames`)
    (for _array_element_2 (`.Frame_3_3FA6ACC844C4C410F8A85F8144DE5AA7` (break `/Game/RLCrowd/Blueprints/Struct/S_AgentStatus2D` _array_element))
      (bind _output_agentmap (break `/Game/RLCrowd/Blueprints/Struct/S_AgentMap` (`|GetArrayItem` (`self.AgentMaps`) _array_index)))
      (`BlueprintMapLibrary.Map_Add` _output_agentmap (`.agent_id_6_F122D5BB44F1D1D3FFC90A80B39A41DF` (break `/Game/RLCrowd/Blueprints/Struct/S_AgentStatus` _array_element_2)) _array_element_2))))

(event `TurnToFrame`
  (params (FrameID :type Integer))
  (bind _output_agentmap (break `/Game/RLCrowd/Blueprints/Struct/S_AgentMap` (`|GetArrayItem` (`self.AgentMaps`) FrameID)))
  (set `self.Frame ID` FrameID)
  (`|ExecutionSequence`
    (:`then_0`
      ;[1 1 1] Clear arrived agents
      (bind _keys (`BlueprintMapLibrary.Map_Keys` (`self.AgentMap`)))
      (for _array_element _keys
        (if (not (`.ReturnValue` (`BlueprintMapLibrary.Map_Find` _output_agentmap _array_element)))
          (bind _value (`BlueprintMapLibrary.Map_Find` (`self.AgentMap`) _array_element))
          (`/Engine/EditorBlueprintResources/StandardMacros.IsValid` _value
            (:`Is Valid`
              (`self.K2_DestroyActor` _value))))))
    (:`then_1`
      ;[1 1 1] Spawn and update agents
      (for _array_element_2 (`.Frame_3_3FA6ACC844C4C410F8A85F8144DE5AA7` (break `/Game/RLCrowd/Blueprints/Struct/S_AgentStatus2D` (`|GetArrayItem` (`self.Frames`) FrameID)))
        (bind (_agent_id _position _velocity _orientation) (break `/Game/RLCrowd/Blueprints/Struct/S_AgentStatus` _array_element_2))
        (bind (_value_2 _returnvalue) (`BlueprintMapLibrary.Map_Find` (`self.AgentMap`) _agent_id))
        (if _returnvalue
          (`/Engine/EditorBlueprintResources/StandardMacros.IsValid` _value_2
            (:`Is Valid`
              (bind _returnvalue_2 (`KismetMathLibrary.Conv_Vector2DToVector` (* _position (100.0 100.0)) 80.0))
              (bind _returnvalue_3 (`KismetMathLibrary.RadiansToDegrees` _orientation))
              (`self.K2_SetActorLocationAndRotation` _value_2 _returnvalue_2 (`KismetMathLibrary.MakeRotator` 0.0 0.0 _returnvalue_3) false false)
              (set `/Game/ThirdPerson/Blueprints/BP_ThirdPersonCharacter.Velocity` _velocity _value_2)))
          (else
            (bind _returnvalue_4 (`|SpawnActorFromClass` "/Game/ThirdPerson/Blueprints/BP_ThirdPersonCharacter.BP_ThirdPersonCharacter_C" (`KismetMathLibrary.MakeTransform` _returnvalue_2 (`KismetMathLibrary.MakeRotator` 0.0 0.0 _returnvalue_3)) "Undefined" "OverrideRootScale" null null))
            (`BlueprintMapLibrary.Map_Add` (`self.AgentMap`) _agent_id _returnvalue_4)
            (`/Engine/EditorBlueprintResources/StandardMacros.IsValid` _returnvalue_4
              (:`Is Valid`
                (set `/Game/ThirdPerson/Blueprints/BP_ThirdPersonCharacter.Velocity` _velocity _returnvalue_4)))))))))

(event `NextFrame`
  ;[1 1 1] 帧跳转
  (bind _output_get (set `self.Frame ID` (`KismetMathLibrary.Clamp` (+ (`self.Frame ID`) 1) 0 (- (`KismetArrayLibrary.Array_Length` (`self.Frames`)) 1))))
  (`self.TurnToFrame` _output_get))

(event `self.ReceiveBeginPlay`
  ;[1 1 1] Main entrance
  (`self.EnableInput` (`GameplayStatics.GetPlayerController` 0)))

(event `Key|SpaceBar`
  (params (Key :type "Key Structure"))
  ;[1 1 1] Main entrance
  (:`Pressed`
    (set `self.RecordDataFileID` (`self.RecordDataFileStartID`))
    (`self.InitOneRecordAndStartMoving`)))

(event `self.ReceiveTick`
  (params (DeltaSeconds :type "Float (single-precision)"))
  ;[1 1 1] Main entrance
  (`/Engine/EditorBlueprintResources/StandardMacros.Gate` true :!label _label
    (:`Exit`
      (`self.NextFrame`)
      (if (== (`self.Frame ID`) (- (`KismetArrayLibrary.Array_Length` (`self.Frames`)) 1))
        (`self.EndMoving`)
        (if (< (`self.RecordDataFileID`) (`self.RecordDataFileEndID`))
          (`/Engine/EditorBlueprintResources/StandardMacros.IncrementInt` (`self.RecordDataFileID`)
            (:`  `
              (`self.InitOneRecordAndStartMoving`))))))))

(event `StartMoving`
  (goto _label :!via `Open`))

(event `LastFrame`
  ;[1 1 1] 帧跳转
  (bind _output_get (set `self.Frame ID` (`KismetMathLibrary.Clamp` (+ (`self.Frame ID`) -1) 0 (- (`KismetArrayLibrary.Array_Length` (`self.Frames`)) 1))))
  (`self.TurnToFrame` _output_get))

(event `EndMoving`
  (goto _label :!via `Close`))

(event `InitOneRecordAndStartMoving`
  (bind _output (`|GetArrayItem` (`self.RecordNames`) (`self.RecordDataFileID`)))
  (`KismetSystemLibrary.PrintString` _output)
  (`self.ReadData` _output)
  (bind _values (`BlueprintMapLibrary.Map_Values` (`self.AgentMap`)))
  (for _array_element _values
    (`/Engine/EditorBlueprintResources/StandardMacros.IsValid` _array_element
      (:`Is Valid`
        (`self.K2_DestroyActor` _array_element))))
  (`BlueprintMapLibrary.Map_Clear` (`self.AgentMap`))
  (`self.TurnToFrame` 0)
  (`self.StartMoving`))

(event `Key|Right`
  (params (Key :type "Key Structure"))
  ;[1 1 1] Interaction
  (:`Pressed`
    (`self.NextFrame`)))

(event `Key|Left`
  (params (Key :type "Key Structure"))
  ;[1 1 1] Interaction
  (:`Pressed`
    (`self.LastFrame`)))

(fn `UserConstructionScript`
  (bind _showgroundplane (`self.ShowGroundPlane`))
  (`parent.UserConstructionScript`)
  (`|ExecutionSequence`
    (:`then_0`
      (bind _output_get (set `self.implicit_env_texture` (`BlueprintMapLibrary.Map_Find` (`self.implicit_env_texture_dict`) (`self.EnvName`))))
      (`MaterialInstanceDynamic.SetTextureParameterValue` (`self.TerrainDynamicMat`) "Texture" _output_get)
      (`LandscapeProxy.SetLandscapeMaterialTextureParameterValue` (`self.Land`) "ImplicitMask" _output_get))
    (:`then_1`
      (`SceneComponent.SetVisibility` (`self.Plane`) _showgroundplane false)
      (`self.SetActorHiddenInGame` (`self.Land`) _showgroundplane))))