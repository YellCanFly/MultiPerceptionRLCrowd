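; Visual and debug layer for a reinforcement-learning crowd agent, built on parent-class sensing and observation functions.
; UpdateVisualization syncs the radius-scaled cylinder, orientation and velocity arrows, and optional terrain observation grid to agent state.
; Clicking toggles marking: highlight, grid, gated per-tick Sense with trace drawing, and a target flag.
; Spawning the flag also binds the agent to BP_EnvRL's info widget, unmarking the previous one.
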(event `self.UpdateVisualization`
  (bind (_implicit_env_obs_range_x _implicit_env_obs_range_y) (`KismetMathLibrary.BreakVector2D` (`self.implicit_env_obs_range`)))
  (bind (_returnvalue_x _returnvalue_y) (`KismetMathLibrary.BreakVector2D` (`self.velocity_to_absolute` (`self.velocity`))))
  (bind _returnvalue (/ (`self.radius`) 0.5))
  (bind (_returnvalue_roll _returnvalue_pitch _returnvalue_yaw) (`KismetMathLibrary.BreakRotator` (`KismetMathLibrary.FindLookAtRotation` (0.0 0.0 0.0) (`KismetMathLibrary.MakeVector` _returnvalue_x _returnvalue_y))))
  ;[1 1 1] Visulazation
  (`|ExecutionSequence`
    (:`then_0`
      (`self.set_agent_location`)
      (`SceneComponent.SetRelativeScale3D` (`self.Cylinder`) (`KismetMathLibrary.MakeVector` _returnvalue _returnvalue 0.1)))
    (:`then_1`
      (`SceneComponent.K2_SetRelativeRotation` (`self.Arrow_Orientation`) (`KismetMathLibrary.MakeRotator` 0.0 0.0 (`KismetMathLibrary.RadiansToDegrees` (`self.orientation`))) false false)
      (`SceneComponent.SetRelativeScale3D` (`self.Arrow_Velocity`) (`KismetMathLibrary.MakeVector` (* (`.OutLength` (`KismetMathLibrary.ToDirectionAndLength2D` (`self.velocity`))) 100.0 0.02) 1.0 1.0))
      (`SceneComponent.K2_SetRelativeRotation` (`self.Arrow_Velocity`) (`KismetMathLibrary.MakeRotator` 0.0 0.0 _returnvalue_yaw) false false))
    (:`then_2`
      (`SceneComponent.SetVisibility` (`self.SM_FrameGrid`) (`self.ShowTerrainObsRange`) false)
      (if (`self.ShowTerrainObsRange`)
        (`SceneComponent.K2_SetRelativeRotation` (`self.SM_FrameGrid`) (`KismetMathLibrary.MakeRotator` 0.0 0.0 (`KismetMathLibrary.RadiansToDegrees` (`self.orientation`))) false false)
        (`SceneComponent.SetRelativeScale3D` (`self.SM_FrameGrid`) (`KismetMathLibrary.MakeVector` _implicit_env_obs_range_x _implicit_env_obs_range_y 0.5))))))

(event `self.SphereCollision.OnClicked`
  (params (TouchedComponent :type "PrimitiveComponent Object Reference") (ButtonPressed :type "Key Structure"))
  ;[1 1 1] Interaction
  (`KismetSystemLibrary.PrintString` "Hello")
  (if (`self.BeMarked`)
    (`self.ResetMark`)
    (else
      (`self.Mark`))))

(event `TestSense`
  ;[1 1 1] Test Func
  (`self.sense`))

(event `Mark`
  ;[1 1 1] Interaction
  (set `self.BeMarked` true)
  (`MeshComponent.SetVectorParameterValueOnMaterials` (`self.Cylinder`) "Color" (`KismetMathLibrary.Conv_LinearColorToVector` (struct :`R` 0.9 :`G` 0.264589 :`B` 0.123484 :`A` 1.0)))
  (set `self.ShowTerrainObsRange` true)
  (`self.StartSensing`)
  (`|ExecutionSequence`
    (:`then_0`
      (`/Engine/EditorBlueprintResources/StandardMacros.IsValid` (`self.TargetFlag`)
        (:`Is Not Valid`
          (if (!= (`self.target_position`) (0.0 0.0) :`ErrorTolerance` 0.005)
            (bind _returnvalue (`|SpawnActorFromClass` "/Game/RLCrowd/Blueprints/BP_Flag.BP_Flag_C" (`KismetMathLibrary.MakeTransform` (`KismetMathLibrary.Conv_Vector2DToVector` (* (`self.target_position`) (100.0 100.0)))) "Undefined" "OverrideRootScale" null null))
            (set `self.TargetFlag` _returnvalue)
            (bind _asbp_env_rl (cast `/Game/RLCrowd/Blueprints/Envs/BP_EnvRL` (`self.env`)))
            (bind _wbp_agentinfo_rl (`/Game/RLCrowd/Blueprints/UI/WBP_Main_RL.WBP_AgentInfo_RL` (`/Game/RLCrowd/Blueprints/Envs/BP_EnvRL.WBP_Main` _asbp_env_rl)))
            (bind _agent (`/Game/RLCrowd/Blueprints/UI/WBP_AgentInfo_RL.Agent` _wbp_agentinfo_rl)
              (:`then`
                (`self.ResetMark` _agent))
              (:`else`
                _))
            (`Widget.SetVisibility` _wbp_agentinfo_rl "SelfHitTestInvisible")
            (set `/Game/RLCrowd/Blueprints/UI/WBP_AgentInfo_RL.Agent` self _wbp_agentinfo_rl)))))))

(event `self.ReceiveTick`
  (params (DeltaSeconds :type "Float (single-precision)"))
  ;[1 1 1] Show Ray cast
  (`parent.ReceiveTick` DeltaSeconds)
  (`/Engine/EditorBlueprintResources/StandardMacros.Gate` true :!label _label
    (:`Exit`
      (`self.sense`))))

(event `StartSensing`
  ;[1 1 1] Show Ray cast
  (set `self.draw_trace_type` "ForOneFrame")
  (goto _label :!via `Open`))

(event `ResetMark`
  (bind _targetflag (`self.TargetFlag`))
  ;[1 1 1] Interaction
  (set `self.BeMarked` false)
  (`MeshComponent.SetVectorParameterValueOnMaterials` (`self.Cylinder`) "Color" (`KismetMathLibrary.Conv_LinearColorToVector` (struct :`R` 0.9 :`G` 0.9 :`B` 0.9 :`A` 1.0)))
  (set `self.ShowTerrainObsRange` false)
  (`self.EndSensing`)
  (`/Engine/EditorBlueprintResources/StandardMacros.IsValid` _targetflag
    (:`Is Valid`
      (`self.K2_DestroyActor` _targetflag)
      (bind _asbp_env_rl (cast `/Game/RLCrowd/Blueprints/Envs/BP_EnvRL` (`self.env`)))
      (bind _wbp_agentinfo_rl (`/Game/RLCrowd/Blueprints/UI/WBP_Main_RL.WBP_AgentInfo_RL` (`/Game/RLCrowd/Blueprints/Envs/BP_EnvRL.WBP_Main` _asbp_env_rl)))
      (`Widget.SetVisibility` _wbp_agentinfo_rl "Hidden")
      (set `/Game/RLCrowd/Blueprints/UI/WBP_AgentInfo_RL.Agent` null _wbp_agentinfo_rl))))

(event `EndSensing`
  ;[1 1 1] Show Ray cast
  (set `self.draw_trace_type` "None")
  (goto _label :!via `Close`))

(event `self.ReceiveDestroyed`
  (bind _targetflag (`self.TargetFlag`))
  ;[1 1 1] On Destroy
  (`/Engine/EditorBlueprintResources/StandardMacros.IsValid` _targetflag
    (:`Is Valid`
      (`self.K2_DestroyActor` _targetflag))))

(fn `print_observation`
  (locals (observation :type "S_FloatArray Structure"))
  (bind (_acceleration_x _acceleration_y) (`KismetMathLibrary.BreakVector2D` (`self.acceleration`)))
  (bind _floats (break `S_FloatArray` (`local.observation`)))
  (bind _floats_2 (break `S_FloatArray` (`local.observation`)))
  (bind _floats_3 (break `S_FloatArray` (`local.observation`)))
  (bind _floats_4 (break `S_FloatArray` (`local.observation`)))
  (bind _floats_5 (break `S_FloatArray` (`local.observation`)))
  (bind _returnvalue (* (`self.num_rays`) 3))
  (bind _returnvalue_2 (* (`self.num_rays`) 3))
  (bind _returnvalue_3 (* (`self.num_rays`) 3))
  (bind _returnvalue_4 (* (`self.num_rays`) 3))
  (bind _returnvalue_5 (`self.get_observation`))
  (set `local.observation` _returnvalue_5)
  (for _index (range (`self.num_rays`))
    (bind _returnvalue_6 (* _index 3))
    (`KismetSystemLibrary.PrintString` (`KismetStringLibrary.Concat_StrStr` "Ray info " (`KismetStringLibrary.Conv_IntToString` _index) ":" (`KismetStringLibrary.Conv_DoubleToString` (`|GetArrayItem` _floats _returnvalue_6)) ", " (`KismetStringLibrary.Conv_DoubleToString` (`|GetArrayItem` _floats (+ _returnvalue_6 1))) ", " (`KismetStringLibrary.Conv_DoubleToString` (`|GetArrayItem` _floats (+ _returnvalue_6 2))))))
  (`KismetSystemLibrary.PrintString` (`KismetStringLibrary.Concat_StrStr` "Weight: " (`KismetStringLibrary.Conv_DoubleToString` (`|GetArrayItem` _floats_3 _returnvalue_4)) (`KismetStringLibrary.Conv_DoubleToString` (`|GetArrayItem` _floats_3 (+ _returnvalue_4 1)))))
  (`KismetSystemLibrary.PrintString` (`KismetStringLibrary.Concat_StrStr` "orientation: " (`KismetStringLibrary.Conv_DoubleToString` (`|GetArrayItem` (`.floats` (break `S_FloatArray` (`local.observation`))) (+ (* (`self.num_rays`) 3) 2)))))
  (`KismetSystemLibrary.PrintString` (`KismetStringLibrary.Concat_StrStr` "velocity:  " (`KismetStringLibrary.Conv_DoubleToString` (`|GetArrayItem` _floats_5 (+ _returnvalue_2 3))) ", " (`KismetStringLibrary.Conv_DoubleToString` (`|GetArrayItem` _floats_5 (+ _returnvalue_2 4)))))
  (`KismetSystemLibrary.PrintString` (`KismetStringLibrary.Concat_StrStr` "target_position_relative: " (`KismetStringLibrary.Conv_DoubleToString` (`|GetArrayItem` _floats_4 (+ _returnvalue 5))) ", " (`KismetStringLibrary.Conv_DoubleToString` (`|GetArrayItem` _floats_4 (+ _returnvalue 6)))))
  (`KismetSystemLibrary.PrintString` (`KismetStringLibrary.Concat_StrStr` "nav_point_relativa: " (`KismetStringLibrary.Conv_DoubleToString` (`|GetArrayItem` _floats_2 (+ _returnvalue_3 7))) ", " (`KismetStringLibrary.Conv_DoubleToString` (`|GetArrayItem` _floats_2 (+ _returnvalue_3 8)))))
  (`KismetSystemLibrary.PrintString` (`KismetStringLibrary.Concat_StrStr` "acceleration: " (`KismetStringLibrary.Conv_DoubleToString` _acceleration_x) ", " (`KismetStringLibrary.Conv_DoubleToString` _acceleration_y)))
  (`KismetSystemLibrary.PrintString` (`KismetStringLibrary.Concat_StrStr` "Angular velocity: " (`KismetStringLibrary.Conv_DoubleToString` (`self.angular_velocity`))))
  (`KismetSystemLibrary.PrintString` (`KismetStringLibrary.Concat_StrStr` "Use Nav Point: " (`KismetStringLibrary.Conv_BoolToString` (`self.use_nav_point`)))))

(fn `UserConstructionScript`)