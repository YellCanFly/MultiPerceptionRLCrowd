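; TCP client actor that bridges the crowd reinforcement-learning environment (BP_EnvRL) to an external peer.
; On BeginPlay it connects using an IP and port that command-line arguments can override.
; Incoming JSON messages either step the environment with actions or reset it with reward and environment settings, replying with observation JSON via a retrying send.
; Eval runs also save agent status after each action for metrics; Enter resends the last step result.
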(event `self.ReceiveBeginPlay`
  (`self.InitIPAndPort`)
  (bind _connectionid (`self.Connect` (`self.ip`) (`self.port`) (delegate `OnDisconnected`) (delegate `OnConnected`) (delegate `OnMessageRecieved`)))
  (set `self.Connection Id` _connectionid)
  (`self.EnableInput` (`GameplayStatics.GetPlayerController` 0))
  (bind _returnvalue (`GameplayStatics.GetActorOfClass` "/Game/RLCrowd/Blueprints/Envs/BP_EnvRL.BP_EnvRL_C"))
  (set `self.BP_EnvRL` _returnvalue))

(event `OnDisconnected`
  (params (ConnectionId :type Integer))
  (`KismetSystemLibrary.PrintString` (`KismetStringLibrary.Concat_StrStr` "Disconnected: " (`KismetStringLibrary.Conv_IntToString` ConnectionId))))

(event `OnConnected`
  (params (ConnectionId :type Integer))
  (`KismetSystemLibrary.PrintString` (`KismetStringLibrary.Concat_StrStr` "Connected: " (`KismetStringLibrary.Conv_IntToString` ConnectionId))))

(event `OnMessageRecieved`
  (params (ConnectionId :type Integer) (Message :type "Array of Byte (by ref)"))
  (bind _bp_envrl (`self.BP_EnvRL`))
  ;[1 1 1] 解析数据类型
  (bind _returnvalue (`self.Message_ReadString` Message (`KismetArrayLibrary.Array_Length` Message)))
  (if (`KismetStringLibrary.EqualEqual_StrStr` _returnvalue)
    (`KismetSystemLibrary.PrintString` "Empty string")
    (else
      (bind (_outjsonobject _returnvalue_2) (`JsonBlueprintFunctionLibrary.FromString` _returnvalue))
      (if _returnvalue_2
        (set `self.recieved_json` _outjsonobject)
        (bind _outvalue (`|GetJsonField` (`self.recieved_json`) "type"))
        (switch `string` _outvalue
          (:`Default`
            (`KismetSystemLibrary.PrintString` "Unknow type"))
          (:`action`
            (`|ExecutionSequence`
              (:`then_0`
                ;[1 1 1] 执行Action
                (bind (_outvalue_2 _returnvalue_3) (`|GetJsonField` (`self.recieved_json`) "actions"))
                (if _returnvalue_3
                  (bind _returnvalue_4 (`EnvBase.step` (`self.BP_EnvRL`) (make `S_Action` _outvalue_2)))
                  (set `self.Obs Reward Done Json Str` _returnvalue_4)
                  (`self.SendDataWithAttempt` 5 (`self.Obs Reward Done Json Str`))))
              (:`then_1`
                ;[1 1 1] 记录eval中的agent状态，用于计算评估指标
                (if (`KismetStringLibrary.EqualEqual_StrStr` (`.env_type` (break `S_EnvConfig` (`EnvBase.env_config` _bp_envrl))) "eval")
                  (`/Game/RLCrowd/Blueprints/Envs/BP_EnvRL.save_current_agents_status` _bp_envrl)))))
          (:`reset`
            (`|ExecutionSequence`
              (:`then_0`
                ;[1 1 1] 配置reward参数
                (bind (_outvalue_3 _returnvalue_5) (`|GetJsonField` (`self.recieved_json`) "reward_info"))
                (if _returnvalue_5
                  (set `EnvBase.reward_config` _outvalue_3 (`self.BP_EnvRL`))))
              (:`then_1`
                ;[1 1 1] Reset环境
                (bind (_outvalue_4 _returnvalue_6) (`|GetJsonField` (`self.recieved_json`) "env_info"))
                (if _returnvalue_6
                  (bind _returnvalue_7 (`EnvBase.reset` (`self.BP_EnvRL`) _outvalue_4))
                  (set `self.Obs Json Str` _returnvalue_7)
                  (`/Game/RLCrowd/Blueprints/Envs/BP_EnvRL.OnEnvReset` (`self.BP_EnvRL`))
                  (`self.SendDataWithAttempt` 5 (`self.Obs Json Str`)))))))
        (else
          (`KismetSystemLibrary.PrintString` "String to json failed"))))))

(event `Sense`
  ;[1 1 1] 测试
  (bind _returnvalue (`EnvBase.get_step_return` (`self.BP_EnvRL`)))
  (`self.SendData` (`self.Connection Id`) (`self.Conv_StringToBytes` _returnvalue)))

(event `Key|Enter`
  (params (Key :type "Key Structure"))
  (:`Pressed`
    (`self.SendDataWithAttempt` 5 (`self.Obs Reward Done Json Str`))))

(fn `InitIPAndPort`
  (bind _returnvalue (`KismetSystemLibrary.GetCommandLine`))
  (`|ExecutionSequence`
    (:`then_0`
      (bind _paramvalue (`self.ParseParam` _returnvalue "ip"))
      (if (`KismetStringLibrary.NotEqual_StrStr` _paramvalue)
        (set `self.ip` _paramvalue)))
    (:`then_1`
      (bind _paramvalue_2 (`self.ParseParam` _returnvalue "port"))
      (if (`KismetStringLibrary.NotEqual_StrStr` _paramvalue_2)
        (set `self.port` (`KismetStringLibrary.Conv_StringToInt` _paramvalue_2))))))

(fn `ParseParam`
  (params (InString :type String) (ParamName :type String))
  (returns (ParamValue :type String))
  (return (`KismetStringLibrary.Replace` (`KismetSystemLibrary.ParseParamValue` InString ParamName) "=")))

(fn `SendDataWithAttempt`
  (params (MaxAttempt :type Integer :default 5) (InStr :type String))
  (returns (Success :type Boolean))
  (locals (CurAttemptNum :type Integer :default 5) (DataStr :type String))
  (set `local.CurAttemptNum` MaxAttempt)
  (set `local.DataStr` InStr)
  (bind _returnvalue (`self.SendData` (`self.Connection Id`) (`self.Conv_StringToBytes` (`local.DataStr`)) :!label _label))
  (if _returnvalue
    (return true)
    (elif (> (`local.CurAttemptNum`) 0)
      (`KismetSystemLibrary.PrintString` (`KismetStringLibrary.Concat_StrStr` "Send data failed, left attempt times=" (`KismetStringLibrary.Conv_IntToString` (`local.CurAttemptNum`))))
      (`/Engine/EditorBlueprintResources/StandardMacros.DecrementInt` (`local.CurAttemptNum`)
        (:`  `
          (goto _label)))
      (else
        (`KismetSystemLibrary.PrintString` "Send data failed")
        (return false)))))

(fn `UserConstructionScript`)